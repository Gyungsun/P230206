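; BP_Character is a character Blueprint that sets up Enhanced Input for movement and look.
; BeginPlay adds a mapping context to the local player subsystem of player controller 0.
; IA_Move adds movement along the skeletal mesh's forward and right vectors at a constant scale, without reading the action value.
; IA_LookUp calls controller pitch and yaw input with zero values, so it produces no rotation.
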(event `self.ReceiveBeginPlay`
  (`/Engine/EditorBlueprintResources/StandardMacros.IsValid` (`GameplayStatics.GetPlayerController` 0)
    (:`Is Valid`
      (`EnhancedInputSubsystemInterface.AddMappingContext` (pcsubsystem `EnhancedInputLocalPlayerSubsystem` (`GameplayStatics.GetPlayerController` 0)) null 0 (struct)))))

(event `EnhancedInput|/Game/Characters/Input/IA_Move`
  (params (ActionValue :type "Vector2D Structure") (ElapsedSeconds :type "Float (double-precision)") (TriggeredSeconds :type "Float (double-precision)") (InputAction :type "InputAction Object Reference" :default "/Game/Characters/Input/IA_Move.IA_Move"))
  ;[1 1 1] move
  (:`Triggered`
    (`self.AddMovementInput` (`SceneComponent.GetForwardVector` (`self.Mesh(SkeletalMesh)`)))
    (`self.AddMovementInput` (`SceneComponent.GetRightVector` (`self.Mesh(SkeletalMesh)`)))))

(event `EnhancedInput|/Game/Characters/Input/IA_LookUp`
  (params (ActionValue :type "Vector2D Structure") (ElapsedSeconds :type "Float (double-precision)") (TriggeredSeconds :type "Float (double-precision)") (InputAction :type "InputAction Object Reference" :default "/Game/Characters/Input/IA_LookUp.IA_LookUp"))
  (:`Triggered`
    (`self.AddControllerPitchInput` 0.0)
    (`self.AddControllerYawInput` 0.0)))

(fn `UserConstructionScript`)